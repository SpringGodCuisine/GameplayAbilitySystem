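; Gameplay ability for the channeled Electrocute spell, which holds the avatar in a shock loop until input is released.
; On activation it captures mouse target data, hides the cursor, faces the hit location and plays the montage.
; The montage's gameplay event starts the shock loop and disables movement; releasing input restores cursor and walking, then ends the ability.
; This graph applies no damage or beam effects.
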(event Ability|EventActivateAbility
  (CallFunction|EnforceImplementsCombatInterface)
  ;[0.1401 0.0888 1] 存储鼠标数据变量
  (bind _datahandle (|TargetDataUnderMouse)
    (:then
      (Class|AuraBeamSpell|StoreMouseDataInfo (Ability|TargetData|GetHitResultfromTargetData _datahandle))
      (Class|AuraBeamSpell|StoreOwnerVariables)
      (Utilities|FlowControl|Sequence
        (:then_0
          (Variables|/Script/Engine.PlayerController|SetbShowMouseCursor (Variables|Default|GetOwnerPlayerController) false)
          (CallFunction|UpdateFacingTarget)
          (|PlayMontageandWaitProxy "None" (Variables|Default|GetMontage_Electrocute) 1.0 "None" false 1.0 0.0 false
            (:then
              (Ability|Tasks|WaitGameplayEvent "(TagName=\"Event.Montage.Electrocute\")" 0
                (:EventReceived
                  (CallFunction|InShockLoop))))))
        (:then_1
          (Ability|Tasks|WaitInputRelease false
            (:OnRelease
              (CallFunction|PreparetoEndAbility)
              (Ability|EndAbility))))))))

(fn EnforceImplementsCombatInterface
  (if (not (Utilities|DoesObjectImplementInterface (Ability|GetAvatarActorfromActorInfo) "/Script/GAS_RPG.CombatInterface"))
    (Ability|EndAbility)))

(fn PreparetoEndAbility
  (Variables|/Script/Engine.PlayerController|SetbShowMouseCursor (Variables|Default|GetOwnerPlayerController) true)
  (Class|CombatInterface|SetinShockLoop(Message) (Ability|GetAvatarActorfromActorInfo) false)
  (Pawn|Components|CharacterMovement|SetMovementMode (Variables|/Script/Engine.Character|GetCharacterMovement (Variables|Default|GetOwnerCharacter)) "MOVE_Walking" 0))

(fn InShockLoop
  (Class|CombatInterface|SetinShockLoop(Message) (Ability|GetAvatarActorfromActorInfo) true)
  (Pawn|Components|CharacterMovement|DisableMovement (Variables|/Script/Engine.Character|GetCharacterMovement (Variables|Default|GetOwnerCharacter))))

(fn UpdateFacingTarget
  (Class|CombatInterface|UpdateFacingTarget(Message) (Ability|GetAvatarActorfromActorInfo) (Variables|Default|GetMouseHitLocation)))